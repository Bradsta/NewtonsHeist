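; Level actor that handles the player's GravityFlip input, changing gravity only while the Hero is not falling.
; It enables its own input on BeginPlay and branches on the NH_Gamemode gravity mode.
; Vertical Only toggles the Hero's gravity direction between up and down.
; Four Way Directional shows the NH_HUD gravity direction widget and disables the pawn's input, leaving the direction choice to that HUD.
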(event EventBeginPlay
  (Input|EnableInput (Game|GetPlayerController 0)))

(event Collision|EventActorBeginOverlap
  (params (OtherActor :type Actor%20Object%20Reference)))

(event EventTick
  (params (DeltaSeconds :type Float%20%28single-precision%29)))

(event Input|ActionEvents|InputActionGravityFlip
  (params (Key :type Key%20Structure :default "AnyKey"))
  (:Pressed
    (bind _ashero (Utilities|Casting|CastToHero (Game|Player|GetPlayerPawn 0)))
    (if (not (AI|Components|NavMovement|IsFalling (Variables|/Script/CustomGravityPlugin.CustomPawn|GetMovementComponent _ashero)))
      (bind _asnh_gamemode (Utilities|Casting|CastToNH_Gamemode (Game|GetGameMode)))
      (switch Utilities|FlowControl|Switch|SwitchonGravityMode (Variables|/Game/Blueprints/NH_Gamemode.NH_Gamemode_C|GetCurrentGravityMode _asnh_gamemode)
        (:NewEnumerator1
          (if (Math|Vector|Equal(Vector) (Class|CustomMovementComponent|GetGravityDirection (Variables|/Script/CustomGravityPlugin.CustomPawn|GetMovementComponent _ashero)) "0, 0,1.000000" 0.0001)
            (Default|SetGravityDirection _ashero "0, 0,-1.000000")
            (else
              (Default|SetGravityDirection _ashero "0, 0,1.000000"))))
        (:NewEnumerator2
          (bind _ashero_2 (Utilities|Casting|CastToHero (Game|Player|GetPlayerPawn 0)))
          (if (not (AI|Components|NavMovement|IsFalling (Variables|/Script/CustomGravityPlugin.CustomPawn|GetMovementComponent _ashero_2)))
            (bind _asnh_hud (Utilities|Casting|CastToNH_HUD (HUD|GetHUD (Game|GetPlayerController 0))))
            (Widget|SetVisibility (Variables|/Game/UserInterface/HUD/NH_HUD.NH_HUD_C|GetGravityDirHUD _asnh_hud) "Visible")
            (Input|DisableInput (Game|Player|GetPlayerPawn 0) (Game|GetPlayerController 0))))))))

(fn ConstructionScript)