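; Actor that lets the player grab, carry and throw physics objects through the Grab Object and Throw Object inputs.
; Pressing grab line-traces forward from the pawn and attaches a newly added physics handle to hits under a mass limit, ignoring Pawn collision.
; Tick keeps the handle target at hold distance ahead of the pawn.
; Releasing grab drops the object and restores Pawn blocking, adding a forward impulse if throw is held.
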(event EventBeginPlay
  (Input|EnableInput (Game|GetPlayerController 0)))

(event Collision|EventActorBeginOverlap
  (params (OtherActor :type Actor%20Object%20Reference)))

(event EventTick
  (params (DeltaSeconds :type Float%20%28single-precision%29))
  (bind _returnvalue (Game|Player|GetPlayerPawn 0))
  (if (Variables|Default|GetPOP%20Physics%20Handle%20Active)
    (if (Variables|Default|GetPOP%20grab%20is%20active)
      (Variables|Default|SetPOP%20handle%20location (+ (Transformation|GetActorLocation _returnvalue) (+ (* (Transformation|GetActorForwardVector _returnvalue) (Variables|Default|GetPOP%20item%20hold%20distance)) "0.000000, 0,0.000000")))
      (Class|PhysicsHandleComponent|SetTargetLocationandRotation (Variables|Default|GetPOP%20Physics%20Handle%20Component) (+ (Variables|Default|GetPOP%20handle%20location) "0, 0,0.000000") "0, 0, 0"))))

(event Input|ActionEvents|InputActionGrabObject
  (params (Key :type Key%20Structure :default "AnyKey"))
  (bind _returnvalue (Game|Player|GetPlayerPawn 0))
  (bind _returnvalue_2 (Transformation|GetActorLocation _returnvalue))
  (:Pressed
    (Variables|Default|SetPOP%20Physics%20Handle%20Active true)
    (bind (_outhit _returnvalue_3) (Collision|LineTraceForObjects _returnvalue_2 (+ _returnvalue_2 (* (Transformation|GetActorForwardVector _returnvalue) (Variables|Default|GetPOP%20Pickup%20distance))) (Utilities|Array|MakeArray (Variables|Default|GetPOP%20object%20types)) false 0 "None"))
    (if _returnvalue_3
      (Variables|Default|SetPOP%20item%20rotation (Transformation|GetWorldRotation (.HitComponent (Collision|BreakHitResult _outhit))))
      (Variables|Default|SetPOP%20grab%20is%20active true)
      (if (< (Physics|GetMass (.HitComponent (Collision|BreakHitResult _outhit))) 5e+02)
        (bind _returnvalue_4 (AddComponent|AddPhysicsHandleComponent))
        (Variables|Default|SetPOP%20Physics%20Handle%20Component _returnvalue_4)
        (Class|PhysicsHandleComponent|SetLinearStiffness (Variables|Default|GetPOP%20Physics%20Handle%20Component) 8e+02)
        (Class|PhysicsHandleComponent|SetInterpolationSpeed (Variables|Default|GetPOP%20Physics%20Handle%20Component) 2e+01)
        (Variables|Default|SetPOP%20object (.HitComponent (Collision|BreakHitResult _outhit)))
        (Class|PhysicsHandleComponent|GrabComponent (Variables|Default|GetPOP%20Physics%20Handle%20Component) (.HitComponent (Collision|BreakHitResult _outhit)) "None" (+ (.Location (Collision|BreakHitResult _outhit)) (* (Transformation|GetActorForwardVector (Game|Player|GetPlayerPawn 0)) "64.000000, 0, 0")) false)
        (Collision|SetCollisionResponsetoChannel (.HitComponent (Collision|BreakHitResult _outhit)) "ECC_Pawn" "ECR_Ignore"))))
  (:Released
    (if (Variables|Default|GetPOP%20grab%20is%20active)
      (Variables|Default|SetPOP%20Physics%20Handle%20Active false)
      (Variables|Default|SetPOP%20grab%20is%20active false)
      (Physics|Components|PhysicsHandle|ReleaseComponent (Variables|Default|GetPOP%20Physics%20Handle%20Component))
      (Class|PrimitiveComponent|WakeRigidBody (.HitComponent (Collision|BreakHitResult _outhit)) "None")
      (if (Variables|Default|GetPOP%20throw%20when%20released)
        (Physics|AddImpulse (.HitComponent (Collision|BreakHitResult _outhit)) (* (Transformation|GetActorForwardVector (Game|Player|GetPlayerPawn 0)) 1e+03) "None" true))
      (Collision|SetCollisionResponsetoChannel (.HitComponent (Collision|BreakHitResult _outhit)) "ECC_Pawn" "ECR_Block"))))

(event Input|ActionEvents|InputActionThrowObject
  (params (Key :type Key%20Structure :default "AnyKey"))
  (:Pressed
    (Variables|Default|SetPOP%20throw%20when%20released true))
  (:Released
    (Variables|Default|SetPOP%20throw%20when%20released false)))

(fn ConstructionScript)