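; Follow camera actor that takes over the first player controller's view and trails a target actor, defaulting to the player pawn.
; On BeginPlay it jumps to the target's location offset along world Y by CameraDistance, using a swept move.
; While FollowPlayer is set, Tick eases toward that point through a brief MoveComponentTo, leaving rotation unchanged.
; A constant-speed move macro is also defined but unused here.
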(event EventTick
  (params (DeltaSeconds :type Float%20%28single-precision%29))
  (bind (_followvector _valid) (CallFunction|GetFollowVector))
  (if (and _valid (Variables|Default|GetFollowPlayer))
    (Utilities|MoveInterpTime _followvector 0.03)))

(event EventBeginPlay
  (CallFunction|Setup)
  (CallFunction|Follow))

(fn ConstructionScript)

(fn Follow
  (bind (_followvector _valid) (CallFunction|GetFollowVector))
  (if _valid
    (Transformation|SetActorLocation _followvector true false)))

(fn GetFollowVector
  (bind _followactor (Variables|Default|GetFollowActor))
  (bind _returnvalue (Transformation|GetActorLocation _followactor))
  (bind (_x _y _z) (Math|Vector|BreakVector _returnvalue))
  (if (Utilities|IsValid _followactor)
    (return (Math|Vector|MakeVector _x (+ _y (Variables|Default|GetCameraDistance)) _z) true)
    (else
      (return "0, 0, 0" false))))

(fn Setup
  (Game|Player|SetViewTargetwithBlend (Game|GetPlayerController 0) self 0.0 "VTBlend_Linear" 0.0 false)
  (if (not (Utilities|IsValid (Variables|Default|GetFollowActor)))
    (Variables|Default|SetFollowActor (Game|Player|GetPlayerPawn 0))))