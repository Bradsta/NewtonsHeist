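; Game mode that owns the hero reference, follow camera, active checkpoint and death/respawn flow.
; BeginPlay finds the Hero, spawns NH_Camera and stores the pawn's start transform as the first checkpoint.
; On death, the hero is teleported aside while the camera follows an emitter easing to the checkpoint, where a new Hero is spawned and possessed.
; SetCheckPoint resets the previous checkpoint; RespawnPlayer swaps heroes instantly at a given transform.
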(event Custom|DeathAndRespawn
  (if (not (Variables|Default|GetIsRespawning))
    (Variables|Default|SetIsRespawning true)
    (bind _returnvalue (Game|SpawnActorfromClass "/Game/Blueprints/RespawnEmitter.RespawnEmitter_C" (Math|Transform|MakeTransform (Transformation|GetActorLocation (Variables|Default|GetPlayer)) "0, 0, 0" "1.000000,1,1") "AlwaysSpawn" 0 0))
    (Variables|/Game/Blueprints/NH_Camera.NH_Camera_C|SetFollowActor (Variables|Default|GetCamera) _returnvalue)
    (Physics|SetSimulatePhysics (Variables|/Script/CustomGravityPlugin.CustomPawn|GetCapsuleComponent (Variables|Default|GetPlayer)) false)
    (Transformation|SetActorLocation (Variables|Default|GetPlayer) "-1000.000000,100.000000,-260.000000" false true) ; We move Kep to a random location.
    (Components|MoveComponentTo (Variables|/Game/Blueprints/RespawnEmitter.RespawnEmitter_C|GetRoot _returnvalue) (.Location (Math|Transform|BreakTransform (Variables|Default|GetCheckPointTransform))) "0, 0, 0" true true 2.0 false)
    (Actor|DestroyActor _returnvalue)
    (bind _returnvalue_2 (Game|SpawnActorfromClass "/Game/Blueprints/Hero.Hero_C" (Variables|Default|GetCheckPointTransform) "AdjustIfPossibleButAlwaysSpawn" 0 0))
    (Actor|DestroyActor (Variables|Default|GetPlayer)) ; Destroy old player.
    (Variables|Default|SetPlayer _returnvalue_2)
    (Variables|/Game/Blueprints/NH_Camera.NH_Camera_C|SetFollowActor (Variables|Default|GetCamera) _returnvalue_2)
    (Pawn|Possess (Game|GetPlayerController 0) _returnvalue_2)
    (Default|Setup (Variables|Default|GetCamera))
    (Variables|Default|SetIsRespawning false)))

(event EventBeginPlay
  (bind _returnvalue (Game|Player|GetPlayerPawn 0))
  (CallFunction|GetPlayer)
  (CallFunction|SetUpCamera)
  (CallFunction|SetCheckPoint (Math|Transform|MakeTransform (Transformation|GetActorLocation _returnvalue) (Pawn|GetControlRotation _returnvalue :!class /Script/Engine.Pawn))))

(fn ConstructionScript)

(fn SetUpCamera
  (if (Utilities|IsValid (Variables|Default|GetPlayer))
    (bind _returnvalue (Game|SpawnActorfromClass "/Game/Blueprints/NH_Camera.NH_Camera_C" (Math|Transform|MakeTransform "0, 0, 0" "0,0.000000, 0") "Undefined" 0 0))
    (Variables|Default|SetCamera _returnvalue)))

(fn GetPlayer
  (bind _outactors (Actor|GetAllActorsOfClass "/Game/Blueprints/Hero.Hero_C"))
  (Variables|Default|SetPlayer (Utilities|Array|Get(acopy) _outactors))
  (return))

(fn RespawnPlayer
  (params (Transform :type Transform))
  ;[1 1 1] Spawns new hero, sets camera to follow new hero, posses it, and finally deletes the old hero.
  (bind _output_get (LocalVariables|SetOldPlayer (Variables|Default|GetPlayer)))
  (bind _returnvalue (Game|SpawnActorfromClass "/Game/Blueprints/Hero.Hero_C" Transform "AdjustIfPossibleButAlwaysSpawn" 0 0))
  (Variables|Default|SetPlayer _returnvalue)
  (Variables|/Game/Blueprints/NH_Camera.NH_Camera_C|SetFollowActor (Variables|Default|GetCamera) _returnvalue)
  (Pawn|Possess (Game|GetPlayerController 0) _returnvalue)
  (Default|Setup (Variables|Default|GetCamera))
  (Actor|DestroyActor _output_get)
  (return))

(fn SetCheckPoint
  (params (Destination :type Transform) (NewCheckPoint :type Check%20Point%20Actor%20Object%20Reference))
  (Variables|Default|SetCheckPointTransform Destination)
  ;[1 1 1] Reset the old checkpoint, then store the new one
  (Utilities|IsValid (Variables|Default|GetLastUsedCheckPoint)
    (:Is%20Valid
      (Default|ResetCheckPoint (Variables|Default|GetLastUsedCheckPoint)))
    (:Is%20Not%20Valid
      _))
  (Variables|Default|SetLastUsedCheckPoint NewCheckPoint)
  (return))