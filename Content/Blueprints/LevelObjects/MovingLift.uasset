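; Moving lift level object that shuttles its static mesh between the origin and a configurable end location and rotation.
; A timeline scaled by TravelTime drives the lerps, then reverses after a stop delay to loop once LIftForward is called.
; Rotating moves apply a special physical material until travel finishes.
; The construction script previews either endpoint via TestEndLocation; safety collider overlap events are empty.
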(event OnComponentBeginOverlap(SafetyCollider)
  (params (OverlappedComponent :type Primitive%20Component%20Object%20Reference) (OtherActor :type Actor%20Object%20Reference) (OtherComp :type Primitive%20Component%20Object%20Reference) (OtherBodyIndex :type Integer) (bFromSweep :type Boolean) (SweepResult :type Hit%20Result%20Structure%20%28by%20ref%29))
  ;[1 1 1] What to do when it overlaps?
)

(event OnComponentEndOverlap(SafetyCollider)
  (params (OverlappedComponent :type Primitive%20Component%20Object%20Reference) (OtherActor :type Actor%20Object%20Reference) (OtherComp :type Primitive%20Component%20Object%20Reference) (OtherBodyIndex :type Integer))
  ;[1 1 1] What to do when it overlaps?
)

(event Custom|LIftForward
  (bind (_direction _driver) (Timeline|LiftTimeline PlayFromStart)
    (:Update
      (Transformation|SetRelativeLocation (Variables|Default|GetStaticMesh) (Math|Vector|Lerp(Vector) "0, 0, 0" (Variables|LiftControls|GetEndLocation) _driver) false false)
      (if (not (Math|Rotator|Equal(Rotator) (Variables|LiftControls|GetEndRotation) (Variables|LiftControls|GetDefaultRotation) 1.0))
        (Transformation|SetRelativeRotation (Variables|Default|GetStaticMesh) (Math|Rotator|Lerp(Rotator) "0, 0, 0" (Variables|LiftControls|GetEndRotation) _driver) false false)
        (Class|PrimitiveComponent|SetPhysMaterialOverride (Variables|Default|GetStaticMesh) (Variables|LiftControls|GetRotatingPhysicsMaterial))))
    (:Finished
      (Class|PrimitiveComponent|SetPhysMaterialOverride (Variables|Default|GetStaticMesh))
      (Utilities|FlowControl|Delay (Variables|LiftControls|GetStopDelay))
      (switch Utilities|FlowControl|Switch|SwitchonETimelineDirection _direction
        (:Forward
          (CallFunction|LIftBackward))
        (:Backward
          (CallFunction|LIftForward))))))

(event Custom|LIftBackward
  (bind (_direction _driver) (Timeline|LiftTimeline ReverseFromEnd)
    (:Update
      (Transformation|SetRelativeLocation (Variables|Default|GetStaticMesh) (Math|Vector|Lerp(Vector) "0, 0, 0" (Variables|LiftControls|GetEndLocation) _driver) false false)
      (if (not (Math|Rotator|Equal(Rotator) (Variables|LiftControls|GetEndRotation) (Variables|LiftControls|GetDefaultRotation) 1.0))
        (Transformation|SetRelativeRotation (Variables|Default|GetStaticMesh) (Math|Rotator|Lerp(Rotator) "0, 0, 0" (Variables|LiftControls|GetEndRotation) _driver) false false)
        (Class|PrimitiveComponent|SetPhysMaterialOverride (Variables|Default|GetStaticMesh) (Variables|LiftControls|GetRotatingPhysicsMaterial))))
    (:Finished
      (Class|PrimitiveComponent|SetPhysMaterialOverride (Variables|Default|GetStaticMesh))
      (Utilities|FlowControl|Delay (Variables|LiftControls|GetStopDelay))
      (switch Utilities|FlowControl|Switch|SwitchonETimelineDirection _direction
        (:Forward
          (CallFunction|LIftBackward))
        (:Backward
          (CallFunction|LIftForward))))))

(event EventBeginPlay
  (Components|Timeline|SetPlayRate (Variables|Default|GetLiftTimeline) (/ 1.0 (Variables|LiftControls|GetTravelTime)))
  (Variables|LiftControls|SetDefaultRotation (Variables|/Script/Engine.SceneComponent|GetRelativeRotation (Variables|Default|GetStaticMesh)))
  (Variables|LiftControls|SetTestEndLocation true))

(fn ConstructionScript
  (Transformation|SetRelativeLocation (Variables|Default|GetStaticMesh) (Math|Vector|SelectVector (Variables|LiftControls|GetEndLocation) "0, 0, 0" (Variables|LiftControls|GetTestEndLocation)) false false)
  (Transformation|SetRelativeRotation (Variables|Default|GetStaticMesh) (Math|Rotator|SelectRotator (Variables|LiftControls|GetEndRotation) "0, 0, 0" (Variables|LiftControls|GetTestEndLocation)) false false))