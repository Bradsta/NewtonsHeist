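; Checkpoint actor that registers itself with NH_Gamemode as the current checkpoint when the Hero overlaps it.
; On BeginPlay it caches the game mode through GetAllActorsOfClass and tints its particle system white.
; Overlap passes the box location and the Hero's control rotation to SetCheckPoint and turns the particles green.
; ResetCheckPoint restores the white color, though nothing in this Blueprint calls it.
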(event EventBeginPlay
  ;[1 1 1] Stores reference of the NH_Gamemode class to later call Respawn() if needed.
  (bind _outactors (Actor|GetAllActorsOfClass "/Game/Blueprints/NH_Gamemode.NH_Gamemode_C"))
  (Variables|Default|SetGame%20Mode%20Actor (Utilities|Array|Get(acopy) _outactors))
  (Effects|Components|ParticleSystem|SetColorParameter (Variables|Default|GetParticleSystem) "InstanceColorScaleOverLife" "(R=1.000000,G=1.000000,B=1.000000,A=1.000000)"))

(event Collision|EventActorBeginOverlap
  (params (OtherActor :type Actor%20Object%20Reference))
  (bind _ashero (Utilities|Casting|CastToHero OtherActor))
  (Default|SetCheckPoint (Variables|Default|GetGame%20Mode%20Actor) (Math|Transform|MakeTransform (Transformation|GetWorldLocation (Variables|Default|GetBox)) (Pawn|GetControlRotation _ashero :!class /Script/Engine.Pawn)) self)
  (Effects|Components|ParticleSystem|SetColorParameter (Variables|Default|GetParticleSystem) "InstanceColorScaleOverLife" "(R=0.000000,G=0.709804,B=0.138638,A=0.000000)"))

(fn ConstructionScript)

(fn ResetCheckPoint
  ;[1 1 1] Reset to Normal Color
  (Effects|Components|ParticleSystem|SetColorParameter (Variables|Default|GetParticleSystem) "InstanceColorScaleOverLife" "(R=1.000000,G=1.000000,B=1.000000,A=0.000000)"))