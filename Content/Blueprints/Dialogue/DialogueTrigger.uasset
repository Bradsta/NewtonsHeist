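; Dialogue trigger that shows a typewriter-style line in the HUD's Newt panel when the Hero first overlaps it, or at BeginPlay if already flagged Triggered.
; While the panel is visible, Tick reveals DialogueTextString by elapsed time over SecondsPerChar.
; Ticks where the revealed length is a multiple of five play a text sound and set one face texture; completing the line sets the other.
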(event EventBeginPlay
  (bind _asnh_hud (Utilities|Casting|CastToNH_HUD (HUD|GetHUD (Game|GetPlayerController 0))))
  (Variables|Default|SetDialogueHUD (Variables|/Game/UserInterface/HUD/NH_HUD.NH_HUD_C|GetDialogueHUD _asnh_hud))
  (if (Variables|Default|GetTriggered)
    (CallFunction|BeginText)))

(event Collision|EventActorBeginOverlap
  (params (OtherActor :type Actor%20Object%20Reference))
  (Utilities|Casting|CastToHero OtherActor)
  (if (not (Variables|Default|GetTriggered))
    (CallFunction|BeginText)))

(event EventTick
  (params (DeltaSeconds :type Float%20%28single-precision%29))
  (bind _isshowing (CallFunction|IsShowing))
  (if _isshowing
    (Utilities|StepText DeltaSeconds)))

(fn ConstructionScript)

(fn IsShowing
  (return (and (Variables|Default|GetTriggered) (Widget|IsVisible (Variables|/Game/UserInterface/HUD/DialogueHUD.DialogueHUD_C|GetNewtPanel (Variables|Default|GetDialogueHUD))))))

(fn BeginText
  (bind _dialoguehud (Variables|Default|GetDialogueHUD))
  (if (Utilities|IsValid _dialoguehud)
    (Widget|SetVisibility (Variables|/Game/UserInterface/HUD/DialogueHUD.DialogueHUD_C|GetNewtPanel _dialoguehud) "Visible")
    (Variables|Default|SetTextTimer 0.0)
    (Variables|Default|SetTriggered true)
    (Variables|Default|SetCompleted false)))