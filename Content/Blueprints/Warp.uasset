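; Warp trigger actor that teleports the Hero to a linked Destination actor when they overlap its Box.
; On BeginPlay it caches the first NH_Gamemode found in the level.
; On overlap with a valid Destination, it calls RespawnPlayer on that game mode with the Destination's location and the Hero's control rotation, because simply setting the actor location did not work well.
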(event OnComponentBeginOverlap(Box)
  (params (OverlappedComponent :type Primitive%20Component%20Object%20Reference) (OtherActor :type Actor%20Object%20Reference) (OtherComp :type Primitive%20Component%20Object%20Reference) (OtherBodyIndex :type Integer) (bFromSweep :type Boolean) (SweepResult :type Hit%20Result%20Structure%20%28by%20ref%29))
  (bind _destination (Variables|Default|GetDestination))
  ;[1 1 1] Calls NH_Gamemode.Respawn() if the collided actor is of type Hero Grav Cameraless. Simply setting the actor location was not working well.
  (bind _ashero (Utilities|Casting|CastToHero OtherActor))
  (Utilities|IsValid _destination
    (:Is%20Valid
      (Default|RespawnPlayer (Variables|Default|GetGameModeActor) (Math|Transform|MakeTransform (Transformation|GetActorLocation _destination) (Pawn|GetControlRotation _ashero :!class /Script/Engine.Pawn))))))

(event EventBeginPlay
  ;[1 1 1] Stores reference of the NH_Gamemode class to later call Respawn() if needed.
  (bind _outactors (Actor|GetAllActorsOfClass "/Game/Blueprints/NH_Gamemode.NH_Gamemode_C"))
  (Variables|Default|SetGameModeActor (Utilities|Array|Get(acopy) _outactors)))

(fn ConstructionScript)