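; Gravity field actor that changes the Hero's gravity direction when the Hero overlaps it.
; It teleports the Hero's capsule to the field's root location when centering is enabled or the Hero's speed exceeds a threshold.
; It zeroes the capsule's physics velocity unless already moving along the new gravity direction, then applies that direction.
; A DoOnce with a short delayed reset prevents rapid retriggering.
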(event Collision|EventActorBeginOverlap
  (params (OtherActor :type Actor%20Object%20Reference))
  (bind _ashero (Utilities|Casting|CastToHero OtherActor))
  (Variables|Default|SetHeroReference _ashero)
  (Utilities|FlowControl|DoOnce false :!label _label
    (:Completed
      (if (or (Variables|Gravity|GetMove%20Player%20to%20Center) (> (Math|Vector|VectorLength (Transformation|GetVelocity (Variables|Default|GetHeroReference))) (Variables|Default|GetSpeedBeforeAutoCenter)))
        (Transformation|SetWorldLocation (Variables|/Script/CustomGravityPlugin.CustomPawn|GetCapsuleComponent (Variables|Default|GetHeroReference)) (Transformation|GetWorldLocation (Variables|Default|GetDefaultSceneRoot self)) false true))
      ;[1 1 1] If already traveling in arrow direction
      (if (Math|Vector|Equal(Vector) (Math|Vector|Normalize (Transformation|GetComponentVelocity (Variables|/Script/CustomGravityPlugin.CustomPawn|GetCapsuleComponent (Variables|Default|GetHeroReference)))) (Math|Vector|Normalize (Variables|Gravity|GetGravity%20Direction)) 0.0001)
        _
        (else
          (Class|PrimitiveComponent|SetAllPhysicsLinearVelocity (Variables|/Script/CustomGravityPlugin.CustomPawn|GetCapsuleComponent (Variables|Default|GetHeroReference)) "0, 0, 0" false)))
      (Default|SetGravityDirection (Variables|Default|GetHeroReference) (Variables|Gravity|GetGravity%20Direction))
      (Utilities|FlowControl|Delay 0.5)
      (goto _label Reset))))

(fn ConstructionScript)