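; Player-controlled 2D Paper flipbook hero for a gravity-flipping game, with running, jumping, pausing and optional gravity-flip and grab abilities spawned as attached actors.
; SetGravityDirection feeds custom gravity to the movement component and swaps the glow material.
; Movement input follows horizontal or vertical world axes according to the actor's up vector.
; Tick updates animation, step sounds, absolute sprite rotation, facing and air-control reset on landing.
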(event Custom|Force%20Enable%20Grab
  ;[1 1 1] Enable Grab ability
  (bind _returnvalue (Game|SpawnActorfromClass "/Game/Blueprints/pickupActor.pickupActor_C" (Math|Conversions|ToTransform(Vector) (Transformation|GetActorLocation)) "AlwaysSpawn" 0 0))
  (bind _output_get (Variables|Default|SetPIckup%20Actor _returnvalue))
  (Transformation|AttachActorToActor _output_get self "None" "SnapToTarget" "SnapToTarget" "SnapToTarget" true))

(event Custom|Force%20Enable%20GravityFlip
  ;[1 1 1] Enable Gravity Flip ability
  (bind _returnvalue (Game|SpawnActorfromClass "/Game/Blueprints/gravityFlipActor.gravityFlipActor_C" (Math|Conversions|ToTransform(Vector) (Transformation|GetActorLocation)) "AlwaysSpawn" 0 0))
  (bind _output_get (Variables|Default|SetGravityFlipActor _returnvalue))
  (Transformation|AttachActorToActor _output_get self "None" "SnapToTarget" "SnapToTarget" "SnapToTarget" true))

(event Custom|Update%20Animation
  (bind _stepsound_2 (Variables|Default|GetstepSound_2))
  (bind _movementcomponent (Variables|Default|GetMovementComponent))
  (bind _stepsound (Variables|Default|GetstepSound))
  (bind _returnvalue (Class|CustomMovementComponent|GetCurrentWalkSpeed _movementcomponent))
  (bind _returnvalue_2 (> _returnvalue 5.0))
  ;[1 1 1] Update Animation
  (if (AI|Components|NavMovement|IsMovingonGround (Variables|Default|GetMovementComponent))
    (Sprite|SetFlipbook (Variables|Default|GetPaperFlipbook) (select _returnvalue_2 "/Game/Sprites/Characters/NewKepler/Sprites/Kepler_Run.Kepler_Run" "/Game/Sprites/Characters/NewKepler/Sprites/Kepler_Idle.Kepler_Idle"))
    (if (and _returnvalue_2 (not (Audio|Components|Audio|IsPlaying _stepsound)))
      (Variables|Default|SetWasWalking true)
      (Audio|Components|Audio|Play _stepsound 0.0)
      (elif (Math|Boolean|ANDBoolean (Variables|Default|GetWasWalking) (not (Audio|Components|Audio|IsPlaying _stepsound_2)) (not _returnvalue_2))
        (Audio|Components|Audio|Play _stepsound_2 0.0)
        (Variables|Default|SetWasWalking false)))
    (else
      (Sprite|SetFlipbook (Variables|Default|GetPaperFlipbook) (select (> (.z (Class|CustomMovementComponent|GetFallingVelocity (Variables|Default|GetMovementComponent))) 0.0) "/Game/Sprites/Characters/NewKepler/Sprites/Kepler_Rising.Kepler_Rising" "/Game/Sprites/Characters/NewKepler/Sprites/Kepler_Rising.Kepler_Rising")))))

(event Custom|Force%20Update%20Air%20Control%20Ratio
  ;[1 1 1] Update Air Control Ratio
  (Variables|/Script/CustomGravityPlugin.CustomMovementComponent|SetAirControlRatio (Variables|Default|GetMovementComponent) (Variables|Default|GetDefault%20Air%20Control%20Ratio)))

(event Custom|Update%20Air%20Control%20Ratio
  ;[1 1 1] Update Air Control Ratio
  (if (AI|Components|NavMovement|IsMovingonGround (Variables|Default|GetMovementComponent))
    (Utilities|FlowControl|DoOnce false :!label _label
      (:Completed
        (Variables|/Script/CustomGravityPlugin.CustomMovementComponent|SetAirControlRatio (Variables|Default|GetMovementComponent) (Variables|Default|GetDefault%20Air%20Control%20Ratio))))
    (else
      (goto _label Reset))))

(event Custom|SetGravityDirection
  (params (New%20Gravity%20Direction :type Vector))
  (bind _paperflipbook (Variables|Default|GetPaperFlipbook))
  ;[1 1 1] Set Gravity Direction
  (if (Math|Vector|Equal(Vector) New%20Gravity%20Direction "0.000000,0.000000,-1.000000" 0.0001)
    (Rendering|Material|SetMaterial _paperflipbook 0 "/Game/Materials/HeroGlowMatt_Green.HeroGlowMatt_Green")
    (else
      (Rendering|Material|SetMaterial _paperflipbook 0 "/Game/Materials/HeroGlowMatt_Green_Blue.HeroGlowMatt_Green_Blue")))
  (Variables|/Script/CustomGravityPlugin.CustomMovementComponent|SetCustomGravityInfo (Variables|Default|GetMovementComponent) (Utilities|Struct|MakeGravityInfo (Variables|Default|GetGravityPower) New%20Gravity%20Direction "EFM_Acceleration" true))
  (Variables|/Script/CustomGravityPlugin.CustomMovementComponent|SetAirControlRatio (Variables|Default|GetMovementComponent) (Variables|Default|GetDefault%20Air%20Control%20Ratio))
  (Utilities|FlowControl|Delay 0.0)
  (Class|CustomMovementComponent|RequestGavityImmediateUpdate (Variables|Default|GetMovementComponent)))

(event Custom|Update%20Flipbook%20Facing%20Direction
  (bind _returnvalue (Transformation|GetActorUpVector))
  (bind _movementcomponent (Variables|Default|GetMovementComponent))
  (bind _returnvalue_2 (Math|Vector|DotProduct _returnvalue "0.000000, 0,1.000000"))
  (bind _returnvalue_3 (Class|CustomMovementComponent|GetMovementVelocity _movementcomponent))
  (bind _returnvalue_4 (Math|Float|Sign(Float) _returnvalue_2))
  ;[1 1 1] Update Flipbook Direction
  (if (!= (.x _returnvalue_3) 0.0)
    (Transformation|SetRelativeScale3D (Variables|Default|GetPaperFlipbook) (Math|Vector|MakeVector (Math|Float|SelectFloat (* (Math|Float|Sign(Float) (.x _returnvalue_3)) _returnvalue_4) 1.0 (!= _returnvalue_4 0.0)) 1.0 1.0))))

(event EventTick
  (params (DeltaSeconds :type Float%20%28single-precision%29))
  (bind _returnvalue (Transformation|GetActorUpVector))
  ;[1 1 1] Event Tick
  (CallFunction|UpdateAnimation)
  (Transformation|SetWorldRotation (Variables|Default|Getflipbook%20root) (Math|Rotator|MakeRotator 0.0 (* (Class|KismetMathLibrary|DegAcos (Math|Vector|DotProduct _returnvalue "0, 0,1.000000")) (Math|Float|Sign(Float) (Math|Vector|DotProduct _returnvalue "-1.000000, 0, 0"))) 0.0) false false)
  (CallFunction|UpdateAirControlRatio)
  (CallFunction|UpdateFlipbookFacingDirection))

(event EventBeginPlay
  (CallFunction|SetGravityDirection "0, 0,-1.000000")
  (Input|EnableInput (Game|GetPlayerController 0))
  (Variables|/Script/Engine.SceneComponent|SetbAbsoluteRotation (Variables|Default|Getflipbook%20root) true)
  (Utilities|FlowControl|Sequence
    (:then_0
      ;[1 1 1] Enable Gravity Flip ability
      (if (Variables|Default|GetisFlipEnabled)
        (bind _returnvalue (Game|SpawnActorfromClass "/Game/Blueprints/gravityFlipActor.gravityFlipActor_C" (Math|Conversions|ToTransform(Vector) (Transformation|GetActorLocation)) "AlwaysSpawn" 0 0))
        (bind _output_get (Variables|Default|SetGravityFlipActor _returnvalue))
        (Transformation|AttachActorToActor _output_get self "None" "SnapToTarget" "SnapToTarget" "SnapToTarget" true)))
    (:then_1
      ;[1 1 1] Enable Grab ability
      (if (Variables|Default|GetisGrabEnabled)
        (bind _returnvalue_2 (Game|SpawnActorfromClass "/Game/Blueprints/pickupActor.pickupActor_C" (Math|Conversions|ToTransform(Vector) (Transformation|GetActorLocation)) "AlwaysSpawn" 0 0))
        (bind _output_get_2 (Variables|Default|SetPIckup%20Actor _returnvalue_2))
        (Transformation|AttachActorToActor _output_get_2 self "None" "SnapToTarget" "SnapToTarget" "SnapToTarget" true)))
    (:then_2
      ;[1 1 1] Add components for step/walking sounds
      (bind _returnvalue_3 (AddComponent|AddAudioComponent false))
      (Variables|Default|SetstepSound _returnvalue_3)
      (bind _returnvalue_4 (AddComponent|AddAudioComponent false))
      (Variables|Default|SetstepSound_2 _returnvalue_4))))

(event Input|ActionEvents|InputActionJump
  (params (Key :type Key%20Structure :default "AnyKey"))
  ;[1 1 1] Handle Jump
  (:Pressed
    (Class|CustomPawn|Jump)
    (if (AI|Components|NavMovement|IsFalling (Variables|Default|GetMovementComponent))
      (Sprite|SetFlipbook (Variables|Default|GetPaperFlipbook) "/Game/Sprites/Characters/NewKepler/Sprites/Kepler_Jump.Kepler_Jump"))))

(event Input|ActionEvents|InputActionPause
  (params (Key :type Key%20Structure :default "AnyKey"))
  ;[1 1 1] Pause
  (:Pressed
    (if (not (Game|IsGamePaused))
      (Utilities|IsValid (Variables|Default|GetPauseMenuReference)
        (:Is%20Valid
          _)
        (:Is%20Not%20Valid
          (bind _returnvalue (UserInterface|CreateWidget "/Game/UserInterface/PauseMenu.PauseMenu_C"))
          (bind _output_get (Variables|Default|SetPauseMenuReference _returnvalue))))
      (UserInterface|Viewport|AddtoViewport _output_get 0)
      (Game|SetGamePaused true)
      (Input|SetInputModeGameandUI (Game|GetPlayerController 0) (Variables|/Game/UserInterface/PauseMenu.PauseMenu_C|GetResumeButton _output_get) "DoNotLock" true))))

(event Input|AxisEvents|InputAxisMoveUp
  (params (AxisValue :type Float%20%28single-precision%29))
  ;[1 1 1] Move Up/Down
  (if (and (!= AxisValue 0.0) (> (Math|Float|Absolute(Float) (Math|Vector|DotProduct (Transformation|GetActorUpVector) "1.000000, 0, 0")) 0.6))
    (Pawn|Input|AddMovementInput "0.000000, 0,1.000000" (* AxisValue (select (AI|Components|NavMovement|IsMovingonGround (Variables|Default|GetMovementComponent)) 1.0 (Variables|/Script/CustomGravityPlugin.CustomMovementComponent|GetAirControlRatio (Variables|Default|GetMovementComponent)))) true)))

(event Input|AxisEvents|InputAxisMoveRight
  (params (AxisValue :type Float%20%28single-precision%29))
  ;[1 1 1] Move Left/Right
  (if (and (!= AxisValue 0.0) (< (Math|Float|Absolute(Float) (Math|Vector|DotProduct (Transformation|GetActorUpVector) "1.000000, 0, 0")) 0.4))
    (Pawn|Input|AddMovementInput "1.000000, 0,0.000000" (* AxisValue (select (AI|Components|NavMovement|IsMovingonGround (Variables|Default|GetMovementComponent)) 1.0 (Variables|/Script/CustomGravityPlugin.CustomMovementComponent|GetAirControlRatio (Variables|Default|GetMovementComponent)))) false)))

(fn ConstructionScript)

(fn SetEnableHero
  (params (Enable :type Boolean))
  (bind _returnvalue (Game|GetPlayerController 0))
  (bind _capsulecomponent (Variables|Default|GetCapsuleComponent))
  (if Enable
    (Physics|SetSimulatePhysics _capsulecomponent true)
    (Input|EnableInput _returnvalue)
    (else
      (Physics|SetSimulatePhysics _capsulecomponent false)
      (Input|DisableInput _returnvalue))))