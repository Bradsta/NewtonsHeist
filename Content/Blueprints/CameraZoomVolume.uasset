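; Trigger volume that changes the game camera's distance when the Hero enters or leaves it.
; It gets the camera from NH_Gamemode on BeginPlay.
; On entry a timeline raises CameraDistance toward CameraDistanceZoom, and on exit a second timeline lowers it toward ExitZoom.
; Timelines serve only as tickers for fixed per-update steps, stopping when the limit is passed or the Overlapped flag flips.
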(event EventBeginPlay
  (bind _asnh_gamemode (Utilities|Casting|CastToNH_Gamemode (Game|GetGameMode)))
  (Variables|Default|SetCamera (Variables|/Game/Blueprints/NH_Gamemode.NH_Gamemode_C|GetCamera _asnh_gamemode)))

(event Collision|EventActorBeginOverlap
  (params (OtherActor :type Actor%20Object%20Reference))
  (bind _camera (Variables|Default|GetCamera))
  (Utilities|Casting|CastToHero OtherActor)
  (Variables|Default|SetOverlapped true)
  (Timeline|Timeline_1 PlayFromStart
    (:Update
      (if (Utilities|IsValid _camera)
        (if (and (< (Variables|/Game/Blueprints/NH_Camera.NH_Camera_C|GetCameraDistance _camera) (Variables|Default|GetCameraDistanceZoom)) (Variables|Default|GetOverlapped))
          (Variables|/Game/Blueprints/NH_Camera.NH_Camera_C|SetCameraDistance _camera (+ (Variables|/Game/Blueprints/NH_Camera.NH_Camera_C|GetCameraDistance _camera) 25.0))
          (else
            (Timeline|Timeline_1 Stop)))))))

(event Collision|EventActorEndOverlap
  (params (OtherActor :type Actor%20Object%20Reference))
  (bind _camera (Variables|Default|GetCamera))
  (Utilities|Casting|CastToHero OtherActor)
  (Variables|Default|SetOverlapped false)
  (Timeline|Timeline_0 PlayFromStart
    (:Update
      (if (Utilities|IsValid _camera)
        (if (and (> (Variables|/Game/Blueprints/NH_Camera.NH_Camera_C|GetCameraDistance _camera) (Variables|Default|GetExitZoom)) (not (Variables|Default|GetOverlapped)))
          (Variables|/Game/Blueprints/NH_Camera.NH_Camera_C|SetCameraDistance _camera (- (Variables|/Game/Blueprints/NH_Camera.NH_Camera_C|GetCameraDistance _camera) 25.0))
          (else
            (Timeline|Timeline_0 Stop)))))))

(fn ConstructionScript)