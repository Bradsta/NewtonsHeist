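; An overlap-triggered actor that switches to another level after playing a fade sequence.
; BeginPlay creates a Level Sequence player for the FadeIn sequence, and a Hero overlap calls BeginLevelSwitch to set the Triggered flag and play it.
; Tick polls that flag and opens the target Level by name once the sequence is no longer playing.
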(event EventBeginPlay
  (bind _returnvalue (Sequencer|Player|CreateLevelSequencePlayer "/Game/Cinematics/Generic/FadeIn.FadeIn"))
  (Variables|Default|SetFadeIn _returnvalue))

(event Collision|EventActorBeginOverlap
  (params (OtherActor :type Actor%20Object%20Reference))
  (Utilities|Casting|CastToHero OtherActor)
  (CallFunction|BeginLevelSwitch))

(event EventTick
  (params (DeltaSeconds :type Float%20%28single-precision%29))
  (if (and (Variables|Default|GetTriggered) (not (Audio|Components|Audio|IsPlaying (Variables|Default|GetFadeIn))))
    (Game|OpenLevel(byName) (Variables|Default|GetLevel))))

(fn ConstructionScript)

(fn BeginLevelSwitch
  (Variables|Default|SetTriggered true)
  (Audio|Components|Audio|Play (Variables|Default|GetFadeIn)))