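; Pulsing laser beam hazard that kills and respawns the Hero, with a death sound, on contact while lit.
; The construction script fits the collision box, beam and dust particles, and end orb to Length.
; After a start offset, a self-rescheduling timer alternates on and off periods, reshowing the orbs one second before relighting as a warning when off-time allows.
; Tick catches a Hero already inside when the beam turns on.
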(event EventBeginPlay
  (|CallParentFunction)
  (Utilities|FlowControl|Delay (Variables|Default|GetInitOffset))
  (Utilities|Time|SetTimerbyFunctionName 0 "ToggleOnOff" (Variables|Default|GetTime%20On)))

(event Collision|EventActorBeginOverlap
  (params (OtherActor :type Actor%20Object%20Reference))
  (bind _ashero (Utilities|Casting|CastToHero OtherActor))
  (Variables|Default|SetOverlapped true)
  (if (Variables|Default|GetTurnedOn)
    (Default|DeathandRespawn (Variables|Default|GetGame%20Mode%20Actor))
    (Audio|SpawnSoundAttached "/Game/Sounds/deathsound_Cue.deathsound_Cue" (Variables|/Script/CustomGravityPlugin.CustomPawn|GetCapsuleComponent _ashero))))

(event Collision|EventActorEndOverlap
  (params (OtherActor :type Actor%20Object%20Reference))
  (Utilities|Casting|CastToHero OtherActor)
  (Variables|Default|SetOverlapped false))

(event EventTick
  (params (DeltaSeconds :type Float%20%28single-precision%29))
  (if (and (Variables|Default|GetOverlapped) (Variables|Default|GetTurnedOn))
    (Variables|Default|SetOverlapped false)
    (bind _ashero (Utilities|Casting|CastToHero (Game|Player|GetPlayerPawn 0)))
    (Default|DeathandRespawn (Variables|Default|GetGame%20Mode%20Actor))
    (Audio|SpawnSoundAttached "/Game/Sounds/deathsound_Cue.deathsound_Cue" (Variables|/Script/CustomGravityPlugin.CustomPawn|GetCapsuleComponent _ashero))))

(fn ConstructionScript
  (bind _returnvalue (Math|Conversions|ToColor(LinearColor) "(R=0.188235,G=0.129412,B=0.270588,A=0.995000)"))
  (bind _dust2 (Variables|Default|GetDust2))
  (bind _box (Variables|Default|GetBox))
  (bind _length (Variables|Default|GetLength))
  (bind _returnvalue_2 (/ _length 2.0))
  (bind _returnvalue_3 (Math|Vector|MakeVector _length 0.0 0.0))
  (bind _particlesysparam (Utilities|Struct|MakeParticleSysParam "DustColor" "PSPT_Color" 0.0 0.0 "0, 0, 0" "0, 0, 0" _returnvalue))
  (bind _returnvalue_4 (Math|Vector|MakeVector _returnvalue_2 0.0 0.0))
  (bind _returnvalue_5 (+ _returnvalue_4 "0,50.000000,50.000000"))
  (bind _particlesysparam_2 (Utilities|Struct|MakeParticleSysParam "Distance" "PSPT_Vector" 0.0 0.0 _returnvalue_5))
  (bind _array (Utilities|Array|MakeArray _particlesysparam_2 _particlesysparam))
  (Components|Box|SetBoxExtent _box (Math|Vector|MakeVector _returnvalue_2 32.0 32.0) true)
  (Transformation|SetRelativeLocation _box _returnvalue_4 false true)
  (Variables|/Script/Engine.ParticleSystemComponent|SetInstanceParameters (Variables|Default|GetLaserEmitter) (Utilities|Array|MakeArray (Utilities|Struct|MakeParticleSysParam "Distance" "PSPT_Scalar" _length)))
  (Variables|/Script/Engine.ParticleSystemComponent|SetInstanceParameters (Variables|Default|GetDust1) _array)
  (Variables|/Script/Engine.ParticleSystemComponent|SetInstanceParameters _dust2 _array)
  (Transformation|SetRelativeLocation _dust2 _returnvalue_3 false false)
  (Transformation|SetRelativeLocation (Variables|Default|GetSphere1) _returnvalue_3 false false))

(fn TurnOff
  (Rendering|SetVisibility (Variables|Default|GetLaserEmitter) false false)
  (Rendering|SetVisibility (Variables|Default|GetSphere) false false)
  (Rendering|SetVisibility (Variables|Default|GetSphere1) false false)
  (Variables|Default|SetTurnedOn false))

(fn Turnon
  (Rendering|SetVisibility (Variables|Default|GetLaserEmitter) true false)
  (Rendering|SetVisibility (Variables|Default|GetSphere) true false)
  (Rendering|SetVisibility (Variables|Default|GetSphere1) true false)
  (Variables|Default|SetTurnedOn true))

(fn ToggleonOff
  (bind _turnedon (Variables|Default|GetTurnedOn))
  (bind _time_off (Variables|Default|GetTime%20Off))
  (if _turnedon
    (CallFunction|TurnOff)
    (else
      (CallFunction|Turnon)))
  (Utilities|Time|SetTimerbyFunctionName 0 "ToggleOnOff" (Math|Float|SelectFloat (Variables|Default|GetTime%20On) (Variables|Default|GetTime%20Off) _turnedon))
  (if (and (>= _time_off 1.0) (not _turnedon))
    (Utilities|Time|SetTimerbyFunctionName 0 "TurnOnOrbs" (- _time_off 1.0))))

(fn TurnonOrbs
  (Rendering|SetVisibility (Variables|Default|GetSphere) true false)
  (Rendering|SetVisibility (Variables|Default|GetSphere1) true false))