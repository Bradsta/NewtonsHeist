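; Trigger volume for a 2D plane that changes the gravity power of a Hero passing through it.
; Overlap begin and end write the enter or exit power to the Hero and its movement component's custom gravity info, keeping the current gravity direction.
; The construction script fits the box, tinted sprite and two particle systems to Width and Height, scaling particle lifetime and spawn area to match.
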(event Collision|EventActorBeginOverlap
  (params (OtherActor :type Actor%20Object%20Reference))
  (bind _entergravitypower (Variables|Default|GetEnterGravityPower))
  (bind _ashero (Utilities|Casting|CastToHero OtherActor))
  (Variables|/Game/Blueprints/Hero.Hero_C|SetGravityPower _ashero _entergravitypower)
  (Variables|/Script/CustomGravityPlugin.CustomMovementComponent|SetCustomGravityInfo (Variables|/Script/CustomGravityPlugin.CustomPawn|GetMovementComponent _ashero) (Utilities|Struct|MakeGravityInfo _entergravitypower (Class|CustomMovementComponent|GetGravityDirection (Variables|/Script/CustomGravityPlugin.CustomPawn|GetMovementComponent _ashero)) "EFM_Acceleration" true)))

(event Collision|EventActorEndOverlap
  (params (OtherActor :type Actor%20Object%20Reference))
  (bind _exitgravitypower (Variables|Default|GetExitGravityPower))
  (bind _ashero (Utilities|Casting|CastToHero OtherActor))
  (Variables|/Game/Blueprints/Hero.Hero_C|SetGravityPower _ashero _exitgravitypower)
  (Variables|/Script/CustomGravityPlugin.CustomMovementComponent|SetCustomGravityInfo (Variables|/Script/CustomGravityPlugin.CustomPawn|GetMovementComponent _ashero) (Utilities|Struct|MakeGravityInfo _exitgravitypower (Class|CustomMovementComponent|GetGravityDirection (Variables|/Script/CustomGravityPlugin.CustomPawn|GetMovementComponent _ashero)) "EFM_Acceleration" true)))

(fn ConstructionScript
  (bind _particlesystem1 (Variables|Default|GetParticleSystem1))
  (bind _box (Variables|Default|GetBox))
  (bind _height (Variables|Default|GetHeight))
  (bind _width (Variables|Default|GetWidth))
  (bind _height_2 (Variables|Default|GetHeight))
  (bind _returnvalue (/ _height_2 2.5e+02))
  (bind _returnvalue_2 (/ _width 2.5e+02))
  (bind _returnvalue_3 (/ _height 2.0))
  (bind _particlesysparam (Utilities|Struct|MakeParticleSysParam "SpawnX" "PSPT_Scalar" _width))
  (bind _particlesysparam_2 (Utilities|Struct|MakeParticleSysParam "Lifetime" "PSPT_Scalar" _returnvalue))
  (bind _particlesysparam_3 (Utilities|Struct|MakeParticleSysParam "SpawnScale" "PSPT_Scalar" _returnvalue_2))
  (bind _array (Utilities|Array|MakeArray _particlesysparam_2 _particlesysparam_3 _particlesysparam))
  ;[1 1 1] Setup Particle system params
  (Variables|/Script/Engine.ParticleSystemComponent|SetInstanceParameters (Variables|Default|GetParticleSystem) _array)
  (Variables|/Script/Engine.ParticleSystemComponent|SetInstanceParameters _particlesystem1 _array)
  (Transformation|SetRelativeLocation _particlesystem1 (Math|Vector|MakeVector 0.0 0.0 (Variables|Default|GetHeight)) false false)
  ;[1 1 1] Set box size and location
  (Transformation|SetRelativeLocation _box (Math|Vector|MakeVector 0.0 0.0 _returnvalue_3) false false)
  (Components|Box|SetBoxExtent _box (Math|Vector|MakeVector (/ (Variables|Default|GetWidth) 2.0) 0.0 _returnvalue_3) true)
  ;[1 1 1] Scale Sprite
  (Transformation|SetRelativeScale3D (Variables|Default|GetPaperSprite) (Math|Vector|MakeVector (/ (Variables|Default|GetWidth) 1e+02) 1.0 (/ (Variables|Default|GetHeight) 1e+02)))
  (Sprite|SetSpriteColor (Variables|Default|GetPaperSprite) (Variables|Default|GetColor)))