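; Patrolling 2D guard character that passes anything it overlaps or hits to its KillComponent.
; BeginPlay seeds the AI Blackboard with patrol targets, home, wait time and whether to sweep; SetInLight updates its light flag.
; Tick picks the walk or stand flipbook and flips facing by X velocity.
; ConeSweep steps the flipbook's child components between pitch bounds, returning true when passing the default angle upward.
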(event Custom|UpdateFlipbook
  ;[1 1 1] Update Flibook
  (if (AI|Components|NavMovement|IsMovingonGround (Variables|Default|GetMovementComponent))
    (Sprite|SetFlipbook (Variables|Default|GetPaperFlipbook) (select (!= (Class|CustomMovementComponent|GetCurrentWalkSpeed (Variables|Default|GetMovementComponent)) 0.0) "/Game/Sprites/Characters/Enemy/NewGuardWalk.NewGuardWalk" "/Game/Sprites/Characters/Enemy/NewGuardStand.NewGuardStand"))
    (else
      (Sprite|SetFlipbook (Variables|Default|GetPaperFlipbook) (select (> (.z (Class|CustomMovementComponent|GetFallingVelocity (Variables|Default|GetMovementComponent))) 0.0) "/Game/Sprites/Characters/Enemy/NewGuardWalk.NewGuardWalk" "/Game/Sprites/Characters/Enemy/NewGuardStand.NewGuardStand")))))

(event Custom|UpdateFacing
  (bind _returnvalue (Transformation|GetActorRotation))
  (bind _roll (Math|Rotator|BreakRotator _returnvalue))
  ;[1 1 1] Update facing direction
  (Math|Float|CompareFloat (.X (Math|Vector|BreakVector (Variables|/Script/Engine.MovementComponent|GetVelocity (Pawn|GetMovementComponent)))) 0.0
    (:>
      (Transformation|SetRelativeRotation (VehicleSound|GetRootComponent) (Math|Rotator|MakeRotator _roll 0.0 0.0) false false))
    (:<
      (Transformation|SetRelativeRotation (VehicleSound|GetRootComponent) (Math|Rotator|MakeRotator _roll 0.0 1.8e+02) false false))))

(event EventTick
  (params (DeltaSeconds :type Float%20%28single-precision%29))
  ;[1 1 1] Tick
  (Variables|Default|SetdeltaTime DeltaSeconds)
  (CallFunction|UpdateFlipbook)
  (CallFunction|UpdateFacing))

(event EventBeginPlay
  (bind _self self)
  (bind _self_2 self)
  (bind _defaultangle (Variables|Visualsweep|GetDefaultAngle))
  (bind _sweep (Variables|Default|GetSweep))
  (bind _returnvalue (AI|GetBlackboard _self_2))
  (bind _returnvalue_2 (AI|GetBlackboard _self))
  ;[1 1 1] Event Begin Play
  ;[1 1 1] Setup Patrol Points
  (AI|Components|Blackboard|SetValueasObject _returnvalue_2 (Variables|Default|GetPoint1) (Variables|Default|GetTarget1))
  (AI|Components|Blackboard|SetValueasObject _returnvalue_2 (Variables|Default|GetPoint2) (Variables|Default|GetTarget2))
  (AI|Components|Blackboard|SetValueasVector (AI|GetBlackboard self) (Variables|Default|GetHomeLocation) (Transformation|GetActorLocation))
  ;[1 1 1] If angles for sweep are too close don't sweep
  (if (and (Math|Float|NearlyEqual(Float) (Variables|Visualsweep|GetUpperBound) _defaultangle 1.0) (Math|Float|NearlyEqual(Float) _defaultangle (Variables|Visualsweep|GetLowerBound) 1.0))
    (AI|Components|Blackboard|SetValueasBool _returnvalue _sweep false)
    (else
      (AI|Components|Blackboard|SetValueasBool _returnvalue _sweep true)))
  (AI|Components|Blackboard|SetValueasFloat (AI|GetBlackboard self) (Variables|Default|GetStopTime) (Variables|Visualsweep|GetwaitTime)))

(event Collision|EventActorBeginOverlap
  (params (OtherActor :type Actor%20Object%20Reference))
  (Default|Kiill (Variables|Default|GetKillComponent) OtherActor))

(event Collision|EventHit
  (params (MyComp :type Primitive%20Component%20Object%20Reference) (Other :type Actor%20Object%20Reference) (OtherComp :type Primitive%20Component%20Object%20Reference) (bSelfMoved :type Boolean) (HitLocation :type Vector :default "0, 0, 0") (HitNormal :type Vector :default "0, 0, 0") (NormalImpulse :type Vector :default "0, 0, 0") (Hit :type Hit%20Result%20Structure%20%28by%20ref%29))
  (Default|Kiill (Variables|Default|GetKillComponent) Other))

(fn ConstructionScript
  (for _array_element (Components|GetChildrenComponents (Variables|Default|GetPaperFlipbook) false)
    (Transformation|SetRelativeRotation _array_element (Math|Rotator|MakeRotator 0.0 (+ (Variables|Visualsweep|GetDefaultAngle) (Variables|Visualsweep|GetlimbRotationSpeed)) 0.0) false false)))

(fn SetinLight
  (params (inLight :type Boolean))
  (AI|Components|Blackboard|SetValueasBool (AI|GetBlackboard self) (Variables|Default|GetInLight) inLight)
  (return))

(fn ResetAttachedRotation
  (for _array_element (Actor|GetAttachedActors)
    (Transformation|SetRelativeRotation (VehicleSound|GetRootComponent _array_element) (Math|Interpolation|RInterpTo (Transformation|GetActorRotation _array_element) "0, 0, 0" 1.0 1.0) false false)))

(fn ConeSweep
  (bind _limbrotationspeed (Variables|Visualsweep|GetlimbRotationSpeed))
  (bind _returnvalue (/ _limbrotationspeed 2.0))
  (LocalVariables|SetchildAngle (.Pitch (Math|Rotator|BreakRotator (Variables|/Script/Engine.SceneComponent|GetRelativeRotation (Utilities|Array|Get(acopy) (Components|GetChildrenComponents (Variables|Default|GetPaperFlipbook) false))))))
  (if (and (Variables|Visualsweep|GetisSweepingUp) (Math|Float|NearlyEqual(Float) (Variables|Visualsweep|GetUpperBound) (LocalVariables|GetchildAngle) (/ (Variables|Visualsweep|GetlimbRotationSpeed) 2.0)))
    (Variables|Visualsweep|SetisSweepingUp false)
    (elif (and (not (Variables|Visualsweep|GetisSweepingUp)) (Math|Float|NearlyEqual(Float) (Variables|Visualsweep|GetLowerBound) (LocalVariables|GetchildAngle) (/ (Variables|Visualsweep|GetlimbRotationSpeed) 2.0)))
      (Variables|Visualsweep|SetisSweepingUp true)))
  (if (and (Variables|Visualsweep|GetisSweepingUp) (Math|Float|NearlyEqual(Float) (- (Variables|Visualsweep|GetDefaultAngle) _returnvalue) (LocalVariables|GetchildAngle) _returnvalue))
    ;[1 1 1] Extra rotate to not get stuck at DefaultAngle
    (for _array_element (Components|GetChildrenComponents (Variables|Default|GetPaperFlipbook) false)
      (Transformation|AddRelativeRotation _array_element (Math|Rotator|MakeRotator 0.0 (Variables|Visualsweep|GetlimbRotationSpeed) 0.0) false false))
    (return true)
    (elif (Variables|Visualsweep|GetisSweepingUp)
      ;[1 1 1] Sweeps up linear
      (for _array_element_2 (Components|GetChildrenComponents (Variables|Default|GetPaperFlipbook) false)
        (Transformation|AddRelativeRotation _array_element_2 (Math|Rotator|MakeRotator 0.0 (Variables|Visualsweep|GetlimbRotationSpeed) 0.0) false false))
      (return false)
      (else
        ;[1 1 1] Sweeps down linear
        (for _array_element_3 (Components|GetChildrenComponents (Variables|Default|GetPaperFlipbook) false)
          (Transformation|AddRelativeRotation _array_element_3 (Math|Rotator|MakeRotator 0.0 (* (Variables|Visualsweep|GetlimbRotationSpeed) -1.0) 0.0) false false))
        (return false)))))