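; Patrol head actor for an AI character that turns to face a target location and can return to a neutral rotation.
; Track rotates the root component toward the look-at rotation of the supplied target, while ResetRotation turns it back to zero world rotation.
; Both events use RInterpTo with fixed delta times and speeds that reach full alpha, so each call snaps rather than eases.
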(event Collision|EventActorBeginOverlap
  (params (OtherActor :type Actor%20Object%20Reference)))

(event EventResetRotation
  ;[1 1 1] Resets rotation
  (Transformation|SetWorldRotation (Variables|Default|GetDefaultSceneRoot) (Math|Interpolation|RInterpTo (Transformation|GetWorldRotation (Variables|Default|GetDefaultSceneRoot)) "0, 0, 0" 3.0 1.0) false false))

(event EventTrack
  (params (targetToTrack :type Vector))
  ;[1 1 1] Track to Location
  (Transformation|SetWorldRotation (Variables|Default|GetDefaultSceneRoot) (Math|Interpolation|RInterpTo (Transformation|GetActorRotation) (Math|Rotator|FindLookatRotation (Transformation|GetActorLocation) targetToTrack) 0.1 1e+01) false false))

(fn ConstructionScript)