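; AI controller for a patrolling character that starts its PatrolManBT behavior tree on BeginPlay.
; It first initializes the PatrolManBB blackboard and stores the pawn's starting position as HomeLocation, with a small Y offset marked as temporary.
; Unconnected nodes that would write two patrol targets to the Point1 and Point2 keys never run, and Tick is unused.
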(event EventBeginPlay
  (bind _blackboardcomponent (Class|AIController|UseBlackboard "/Game/Blueprints/AICharacter/PatrolManBB.PatrolManBB"))
  (AI|Components|Blackboard|SetValueasVector _blackboardcomponent (Variables|Default|GetHomeLocation) (- (Transformation|GetActorLocation (Pawn|GetControlledPawn)) "0,25.000000, 0"))
  (AI|RunBehaviorTree "/Game/Blueprints/AICharacter/PatrolManBT.PatrolManBT"))

(event EventTick
  (params (DeltaSeconds :type Float%20%28single-precision%29)))

(fn ConstructionScript)