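; Patrol arm attached to a PatrolMan AI character, carrying lights that detect the Hero.
; Inner, middle and outer light volumes share overlap logic that sets InLight on the owning PatrolMan to notify its Behavior Tree; exiting any volume clears it.
; Track and ResetRotation use RInterpTo to turn the arm toward a target or back to zero rotation.
; Sweep applies alternating pitch steps in one loop, with debug printing.
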(event OnComponentEndOverlap(light_outside)
  (params (OverlappedComponent :type Primitive%20Component%20Object%20Reference) (OtherActor :type Actor%20Object%20Reference) (OtherComp :type Primitive%20Component%20Object%20Reference) (OtherBodyIndex :type Integer))
  ;[1 1 1] Notifies Behavior Tree when player exits light
  (Utilities|Casting|CastToHero OtherActor)
  (bind _aspatrol_man (Utilities|Casting|CastToPatrolMan (Components|GetOwner (Transformation|GetAttachParent (VehicleSound|GetRootComponent)))))
  (Default|SetinLight _aspatrol_man false))

(event OnComponentBeginOverlap(light_inside)
  (params (OverlappedComponent :type Primitive%20Component%20Object%20Reference) (OtherActor :type Actor%20Object%20Reference) (OtherComp :type Primitive%20Component%20Object%20Reference) (OtherBodyIndex :type Integer) (bFromSweep :type Boolean) (SweepResult :type Hit%20Result%20Structure%20%28by%20ref%29))
  ;[1 1 1] Notifies Behavior Tree if Hero touched by light
  (Utilities|Casting|CastToHero (stale OnComponentBeginOverlap(light_outside) OtherActor))
  (bind _aspatrol_man (Utilities|Casting|CastToPatrolMan (Components|GetOwner (Transformation|GetAttachParent (VehicleSound|GetRootComponent)))))
  (Default|SetinLight _aspatrol_man true))

(event OnComponentBeginOverlap(light_mid)
  (params (OverlappedComponent :type Primitive%20Component%20Object%20Reference) (OtherActor :type Actor%20Object%20Reference) (OtherComp :type Primitive%20Component%20Object%20Reference) (OtherBodyIndex :type Integer) (bFromSweep :type Boolean) (SweepResult :type Hit%20Result%20Structure%20%28by%20ref%29))
  ;[1 1 1] Notifies Behavior Tree if Hero touched by light
  (Utilities|Casting|CastToHero (stale OnComponentBeginOverlap(light_outside) OtherActor))
  (bind _aspatrol_man (Utilities|Casting|CastToPatrolMan (Components|GetOwner (Transformation|GetAttachParent (VehicleSound|GetRootComponent)))))
  (Default|SetinLight _aspatrol_man true))

(event OnComponentBeginOverlap(light_outside)
  (params (OverlappedComponent :type Primitive%20Component%20Object%20Reference) (OtherActor :type Actor%20Object%20Reference) (OtherComp :type Primitive%20Component%20Object%20Reference) (OtherBodyIndex :type Integer) (bFromSweep :type Boolean) (SweepResult :type Hit%20Result%20Structure%20%28by%20ref%29))
  ;[1 1 1] Notifies Behavior Tree if Hero touched by light
  (Utilities|Casting|CastToHero OtherActor)
  (bind _aspatrol_man (Utilities|Casting|CastToPatrolMan (Components|GetOwner (Transformation|GetAttachParent (VehicleSound|GetRootComponent)))))
  (Default|SetinLight _aspatrol_man true))

(event OnComponentEndOverlap(light_mid)
  (params (OverlappedComponent :type Primitive%20Component%20Object%20Reference) (OtherActor :type Actor%20Object%20Reference) (OtherComp :type Primitive%20Component%20Object%20Reference) (OtherBodyIndex :type Integer))
  ;[1 1 1] Notifies Behavior Tree when player exits light
  (Utilities|Casting|CastToHero (stale OnComponentEndOverlap(light_outside) OtherActor))
  (bind _aspatrol_man (Utilities|Casting|CastToPatrolMan (Components|GetOwner (Transformation|GetAttachParent (VehicleSound|GetRootComponent)))))
  (Default|SetinLight _aspatrol_man false))

(event OnComponentEndOverlap(light_inside)
  (params (OverlappedComponent :type Primitive%20Component%20Object%20Reference) (OtherActor :type Actor%20Object%20Reference) (OtherComp :type Primitive%20Component%20Object%20Reference) (OtherBodyIndex :type Integer))
  ;[1 1 1] Notifies Behavior Tree when player exits light
  (Utilities|Casting|CastToHero (stale OnComponentEndOverlap(light_outside) OtherActor))
  (bind _aspatrol_man (Utilities|Casting|CastToPatrolMan (Components|GetOwner (Transformation|GetAttachParent (VehicleSound|GetRootComponent)))))
  (Default|SetinLight _aspatrol_man false))

(event EventTrack
  (params (targetToTrack :type Vector))
  ;[1 1 1] Tracks target
  (Transformation|SetWorldRotation (VehicleSound|GetRootComponent) (Math|Interpolation|RInterpTo (Transformation|GetActorRotation) (Math|Rotator|FindLookatRotation (Transformation|GetActorLocation) targetToTrack) 0.1 1e+01) false false))

(event EventResetRotation
  ;[1 1 1] Resets rotation
  (Transformation|SetWorldRotation (VehicleSound|GetRootComponent) (Math|Interpolation|RInterpTo (Transformation|GetWorldRotation (Variables|Default|GetDefaultSceneRoot)) "0, 0, 0" 1.0 1.0) false false))

(fn ConstructionScript)

(fn Sweep
  (LocalVariables|SetinitialRotation (Transformation|GetActorRotation))
  (for _index (range 0 2)
    (Development|PrintString (Utilities|String|ToString(Float) (Math|Float|Power -1.0 (Math|Conversions|ToFloat(Integer) _index))))
    (Transformation|SetWorldRotation (VehicleSound|GetRootComponent) (Math|Interpolation|RInterpTo (LocalVariables|GetinitialRotation) (Math|Rotator|CombineRotators (LocalVariables|GetinitialRotation) (Math|Rotator|MakeRotator 0.0 (* (Math|Float|Power -1.0 (Math|Conversions|ToFloat(Integer) _index)) 1e+01) 0.0)) (Utilities|Time|GetWorldDeltaSeconds) 1.0) false false)))