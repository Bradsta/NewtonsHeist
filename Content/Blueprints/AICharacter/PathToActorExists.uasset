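; Behavior tree decorator that checks whether the AI pawn has a navigation path to the actor it is set to follow.
; Its AI condition check runs a synchronous pathfind from the controlled pawn's location to the TargetToFollow blackboard actor and passes if the resulting path is valid.
; The event graph holds only an unused, disconnected copy of the same query.
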(fn PerformConditionCheckAI
  (params (OwnerController :type AI%20Controller%20Object%20Reference) (ControlledPawn :type Pawn%20Object%20Reference))
  (bind _returnvalue (Class|NavigationSystem|FindPathtoActorSynchronously (Transformation|GetActorLocation ControlledPawn) (AI|BehaviorTree|GetBlackboardValueasActor (Variables|Default|GetTargetToFollow)) 5e+01))
  (return (Utilities|IsValid _returnvalue)))