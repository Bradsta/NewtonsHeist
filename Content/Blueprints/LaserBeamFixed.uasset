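; LaserBeamFixed is a fixed-length laser beam actor, set up entirely in the construction script with no active event logic.
; A Length variable sizes and centers the box along local X and moves Sphere1 and Dust2 to the far end.
; It also feeds "Distance" particle instance parameters, as a scalar for the laser emitter and a half-length-based vector for both dust emitters.
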(event EventBeginPlay)

(event Collision|EventActorBeginOverlap
  (params (OtherActor :type Actor%20Object%20Reference)))

(event EventTick
  (params (DeltaSeconds :type Float%20%28single-precision%29)))

(fn ConstructionScript
  (bind _dust2 (Variables|Default|GetDust2))
  (bind _box (Variables|Default|GetBox))
  (bind _length (Variables|Default|GetLength))
  (bind _returnvalue (/ _length 2.0))
  (bind _returnvalue_2 (Math|Vector|MakeVector _length 0.0 0.0))
  (bind _returnvalue_3 (Math|Vector|MakeVector _returnvalue 0.0 0.0))
  (bind _returnvalue_4 (+ _returnvalue_3 "0,50.000000,50.000000"))
  (bind _particlesysparam (Utilities|Struct|MakeParticleSysParam "Distance" "PSPT_Vector" 0.0 0.0 _returnvalue_4))
  (bind _array (Utilities|Array|MakeArray _particlesysparam))
  (Components|Box|SetBoxExtent _box (Math|Vector|MakeVector _returnvalue 32.0 32.0) true)
  (Transformation|SetRelativeLocation _box _returnvalue_3 false true)
  (Variables|/Script/Engine.ParticleSystemComponent|SetInstanceParameters (Variables|Default|GetLaserEmitter) (Utilities|Array|MakeArray (Utilities|Struct|MakeParticleSysParam "Distance" "PSPT_Scalar" _length)))
  (Variables|/Script/Engine.ParticleSystemComponent|SetInstanceParameters (Variables|Default|GetDust1) _array)
  (Variables|/Script/Engine.ParticleSystemComponent|SetInstanceParameters _dust2 _array)
  (Transformation|SetRelativeLocation _dust2 _returnvalue_2 false false)
  (Transformation|SetRelativeLocation (Variables|Default|GetSphere1) _returnvalue_2 false false))